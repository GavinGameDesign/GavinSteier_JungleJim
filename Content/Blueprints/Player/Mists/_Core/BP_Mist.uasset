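; BP_Mist is a trigger volume that transforms the player into another pawn type, set by its MistType, when the player capsule overlaps it.
; It skips players already of that class, then asks BP_GM_ThirdPerson to perform the MistTransform with the chosen transition type.
; The new pawn spawns at the mist facing the camera yaw and is launched along a custom direction or an up-and-backward default.
; A DoOnce gate re-arms on a timer after each use.
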(event OnComponentBeginOverlap(Sphere)
  (params (OverlappedComponent :type Primitive%20Component%20Object%20Reference) (OtherActor :type Actor%20Object%20Reference) (OtherComp :type Primitive%20Component%20Object%20Reference) (OtherBodyIndex :type Integer) (bFromSweep :type Boolean) (SweepResult :type Hit%20Result%20Structure%20%28by%20ref%29))
  (bind _returnvalue (Game|GetPlayerController 0))
  (bind _returnvalue_2 (Game|GetPlayerCameraManager 0))
  (bind _returnvalue_3 (Game|GetPlayerController 0))
  (bind _returnvalue_4 (Transformation|GetActorTransform))
  (bind _returnvalue_5 (Pawn|GetControlledPawn _returnvalue))
  (bind _returnvalue_6 (Camera|GetCameraRotation _returnvalue_2))
  (bind _returnvalue_7 (Pawn|GetControlledPawn _returnvalue_3))
  (bind _returnvalue_8 (Transformation|GetActorRotation _returnvalue_7))
  (bind _returnvalue_9 (Math|Rotator|MakeRotator (.roll _returnvalue_8) (.pitch _returnvalue_8) (.yaw _returnvalue_6)))
  (bind _returnvalue_10 (Math|Transform|MakeTransform (.location _returnvalue_4) _returnvalue_9))
  (if (Components|ComponentHasTag OtherComp "PlayerCapsule")
    (if (not (CallFunction|IsPlayerAlreadyThatClass))
      (Utilities|FlowControl|DoOnce false
        (:Completed
          (bind _asbp_gm_third_person (Utilities|Casting|CastToBP_GM_ThirdPerson (Game|GetGameMode)))
          (if (Class|KismetMathLibrary|EqualExactlyVectorVector (Variables|Default|GetcustomLaunchDirection) "0, 0, 0")
            (CallFunction|TransformIntoActor _asbp_gm_third_person _returnvalue_10 (* (Math|Vector|Normalize (Math|Vector|Lerp(Vector) (Transformation|GetActorUpVector _returnvalue_5) (* (Transformation|GetActorForwardVector _returnvalue_5) -1.0) 0.3)) (Variables|Default|GetmistLaunchIntensity)))
            (else
              (CallFunction|TransformIntoActor _asbp_gm_third_person _returnvalue_10 (* (Math|Vector|Normalize (Variables|Default|GetcustomLaunchDirection)) (Variables|Default|GetmistLaunchIntensity)))))
          (Utilities|Time|SetTimerbyFunctionName 0 "ResetMist" 4.0))))))

(event Custom|ResetMist
  (bind _returnvalue (Game|GetPlayerController 0))
  (bind _returnvalue_2 (Game|GetPlayerCameraManager 0))
  (bind _returnvalue_3 (Game|GetPlayerController 0))
  (bind _returnvalue_4 (Transformation|GetActorTransform))
  (bind _returnvalue_5 (Pawn|GetControlledPawn _returnvalue))
  (bind _returnvalue_6 (Camera|GetCameraRotation _returnvalue_2))
  (bind _returnvalue_7 (Pawn|GetControlledPawn _returnvalue_3))
  (bind _returnvalue_8 (Transformation|GetActorRotation _returnvalue_7))
  (bind _returnvalue_9 (Math|Rotator|MakeRotator (.roll _returnvalue_8) (.pitch _returnvalue_8) (.yaw _returnvalue_6)))
  (bind _returnvalue_10 (Math|Transform|MakeTransform (.location _returnvalue_4) _returnvalue_9))
  (Utilities|FlowControl|DoOnce false) ; enters at Reset
)

(fn ConstructionScript)

(fn IsPlayerAlreadyThatClass
  (bind _returnvalue (Game|GetPlayerController 0))
  (bind _returnvalue_2 (Pawn|GetControlledPawn _returnvalue))
  (switch Utilities|FlowControl|Switch|SwitchonE_MistTypes (Variables|Default|GetmistType)
    (:NewEnumerator0
      (Utilities|Casting|CastToBP_PlayerBase _returnvalue_2
        (:then
          (return true))
        (:CastFailed
          (return false))))
    (:NewEnumerator1
      (Utilities|Casting|CastToBP_MistActorBase _returnvalue_2
        (:then
          (return true))
        (:CastFailed
          (return false))))
    (:NewEnumerator2
      (Utilities|Casting|CastToBP_MistActorPaperAirplane _returnvalue_2
        (:then
          (return true))
        (:CastFailed
          (return false))))))

(fn TransformIntoActor
  (params (GameMode :type BP%20GM%20Third%20Person%20Object%20Reference) (spawnTransform :type Transform) (mistLaunchVelocity :type Vector))
  (switch Utilities|FlowControl|Switch|SwitchonE_MistTransitionType (Variables|Default|GetmistTransitionType)
    (:NewEnumerator0
      (Default|MistTransform GameMode (Variables|Default|GetmistType) "NewEnumerator0" spawnTransform mistLaunchVelocity))
    (:NewEnumerator1
      (Default|MistTransform GameMode (Variables|Default|GetmistType) "NewEnumerator1" spawnTransform mistLaunchVelocity))
    (:NewEnumerator2
      (Default|MistTransform GameMode (Variables|Default|GetmistType) "NewEnumerator2" spawnTransform mistLaunchVelocity))))